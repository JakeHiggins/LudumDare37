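; Throwable pillow actor for the floor-is-lava game that the player picks up and throws with the Throw input.
; Overlapping anything other than the floor enables input and pickup, which attaches the actor to the player with collision off.
; Throwing enables physics on the Pillow and applies a forward-and-upward impulse, without detaching the actor.
; Floor overlap starts a Tick timer that stops physics after BounceDuration and disables Sphere collision.
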(event `self.ReceiveTick`
  (params (DeltaSeconds :type "Float (single-precision)"))
  (if (`self.HitGround`)
    (bind _output_get (set `self.BounceTime` (+ DeltaSeconds (`self.BounceTime`))))
    (if (> _output_get (`self.BounceDuration`))
      (`PrimitiveComponent.SetSimulatePhysics` (`self.Pillow`) false)
      (set `self.HitGround` false)
      (set `self.BounceTime` 0.0)
      (`PrimitiveComponent.SetCollisionEnabled` (`self.Sphere`) "NoCollision"))))

(event `self.ReceiveActorBeginOverlap`
  (params (OtherActor :type "Actor Object Reference"))
  (cast `/Game/FloorIsLava/Blueprints/Floor_Blueprint` OtherActor
    (:`then`
      (set `self.HitGround` true))
    (:`CastFailed`
      (`KismetSystemLibrary.PrintString` "Press E To Pick Up Pillow")
      (set `self.CanPlayerPickup` true)
      (`self.EnableInput` (`GameplayStatics.GetPlayerController` 0)))))

(event `InputAction|Throw`
  (params (Key :type "Key Structure" :default "AnyKey"))
  (bind _returnvalue (`GameplayStatics.GetPlayerCharacter` 0))
  (bind _returnvalue_2 (`self.GetActorForwardVector` (`GameplayStatics.GetPlayerCharacter` 0)))
  (:`Pressed`
    (if (`self.PlayerHolding`)
      (`KismetSystemLibrary.PrintString` "Throw Billow")
      (`PrimitiveComponent.SetCollisionEnabled` (`self.Sphere`) "NoCollision")
      (`PrimitiveComponent.SetCollisionEnabled` (`self.Pillow`) "QueryAndPhysics")
      (`SceneComponent.SetVisibility` (`self.Pillow`) true false)
      (`PrimitiveComponent.SetSimulatePhysics` (`self.Pillow`) true)
      (set `self.PlayerHolding` false)
      (`KismetSystemLibrary.PrintString` (`KismetStringLibrary.Conv_VectorToString` _returnvalue_2))
      (`PrimitiveComponent.AddImpulse` (`self.Pillow`) (* (+ _returnvalue_2 (0.0 0.0 1.0)) 15000.0) "None" false)
      (set `self.Thrown` true)
      (elif (`self.CanPlayerPickup`)
        (set `self.PlayerHolding` true)
        (`KismetSystemLibrary.PrintString` "You Got pillow")
        (`self.K2_SetActorLocation` (+ (+ (`self.K2_GetActorLocation` _returnvalue) (`self.GetActorForwardVector` _returnvalue)) (150.0 0.0 0.0)))
        (`self.K2_AttachToActor` _returnvalue "None" "KeepWorld" "KeepWorld" "KeepWorld")
        (`PrimitiveComponent.SetCollisionEnabled` (`self.Pillow`) "NoCollision")
        (`PrimitiveComponent.SetCollisionEnabled` (`self.Sphere`) "NoCollision")
        (set `self.CanPlayerPickup` false)))))

(fn `UserConstructionScript`)