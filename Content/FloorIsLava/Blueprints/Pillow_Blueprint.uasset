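; Pillow actor for the FloorIsLava game that can be thrown while its PlayerHolding flag is set.
; The E key or Throw action enables mesh physics, adds a small unscaled force from the player controller's forward vector plus a fixed Y offset, then clears the flag.
; Mesh overlap only prints a debug greeting, and nothing here sets the holding flag to true.
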(event `self.StaticMeshComponent.OnComponentBeginOverlap`
  (params (OverlappedComponent :type "PrimitiveComponent Object Reference") (OtherActor :type "Actor Object Reference") (OtherComp :type "PrimitiveComponent Object Reference") (OtherBodyIndex :type Integer) (bFromSweep :type Boolean) (SweepResult :type "HitResult Structure (by ref)"))
  (`KismetSystemLibrary.PrintString` "Hello"))

(event `Key|E`
  (params (Key :type "Key Structure" :default "AnyKey"))
  (:`Pressed`
    (if (`self.PlayerHolding`) :!label _label
      (`PrimitiveComponent.SetSimulatePhysics` (`self.StaticMeshComponent`) true)
      (`PrimitiveComponent.AddForce` (`self.StaticMeshComponent`) (+ (`self.GetActorForwardVector` (`GameplayStatics.GetPlayerController` 0)) (0.0 1.0 0.0)) "None" false)
      (set `self.PlayerHolding` false))))

(event `InputAction|Throw`
  (params (Key :type "Key Structure" :default "AnyKey"))
  (:`Pressed`
    (goto _label)))

(fn `UserConstructionScript`)