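; Throwable pillow for the Floor Is Lava game that the player picks up, carries and throws.
; Overlap enables pickup if the player's hands are empty, and the Throw input attaches the pillow to the character with collision off.
; Holding Throw oscillates launch strength between limits, and release sets physics velocity forward and upward.
; Touching the lava floor flags a timed physics freeze, which Tick advances only during throw charging.
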(event `self.ReceiveActorBeginOverlap`
  (params (OtherActor :type "Actor Object Reference"))
  ;[1 1 1] Determines if the pillow is in connection with the lava
  (cast `/Game/FloorIsLava/Blueprints/Floor_Blueprint` OtherActor
    (:`then`
      (set `self.HitGround` true))
    (:`CastFailed`
      ;[1 1 1] Determines if the player is holding a pillow
      (bind _outactors (`GameplayStatics.GetAllActorsOfClass` "/Game/ThirdPersonBP/Blueprints/ThirdPersonCharacter.ThirdPersonCharacter_C"))
      (bind _holding_object (`/Game/ThirdPersonBP/Blueprints/ThirdPersonCharacter.GetHoldingObject` (`KismetArrayLibrary.Array_Get` _outactors)))
      (if (not _holding_object)
        ;[1 1 1] Allow player to pick up pillow
        (`KismetSystemLibrary.PrintString` "Press E To Pick Up Pillow")
        (set `self.CanPlayerPickup` true)
        (`self.EnableInput` (`GameplayStatics.GetPlayerController` 0))))))

(event `self.ReceiveTick`
  (params (DeltaSeconds :type "Float (single-precision)"))
  (if (`self.CharginThrow`)
    (`KismetSystemLibrary.PrintString` (`KismetStringLibrary.Conv_DoubleToString` (`self.CurrentImpulse`)))
    (if (`self.IncreaseImpulse`)
      (bind _output_get (set `self.CurrentImpulse` (+ (`self.CurrentImpulse`) (`self.ImpusleIncrement`))))
      (if (>= _output_get (`self.MaximumImpulse`))
        (set `self.IncreaseImpulse` false))
      (else
        (bind _output_get_2 (set `self.CurrentImpulse` (- (`self.CurrentImpulse`) (`self.ImpusleIncrement`))))
        (if (<= _output_get_2 (`self.MinimumImpulse`))
          (set `self.IncreaseImpulse` true))))
    (if (`self.HitGround`)
      (bind _output_get_3 (set `self.BounceTime` (+ DeltaSeconds (`self.BounceTime`))))
      (if (> _output_get_3 (`self.BounceDuration`))
        (`PrimitiveComponent.SetSimulatePhysics` (`self.Pillow`) false)
        (set `self.HitGround` false)
        (set `self.BounceTime` 0.0)))))

(event `InputAction|Throw`
  (params (Key :type "Key Structure" :default "AnyKey"))
  (bind _returnvalue (`GameplayStatics.GetPlayerCharacter` 0))
  (bind _pillow (`self.Pillow`))
  (:`Pressed`
    (if (`self.PlayerHolding`)
      (set `self.CharginThrow` true)
      (elif (`self.CanPlayerPickup`)
        (`self.K2_SetActorLocation` (+ (`self.K2_GetActorLocation` _returnvalue) (* (`self.GetActorForwardVector` _returnvalue) 150.0)))
        (`self.K2_AttachToActor` _returnvalue "None" "KeepWorld" "KeepWorld" "KeepWorld")
        (`PrimitiveComponent.SetCollisionEnabled` (`self.Pillow`) "NoCollision")
        (`PrimitiveComponent.SetCollisionEnabled` (`self.Sphere`) "NoCollision")
        (set `self.CanPlayerPickup` false)
        (bind _outactors (`GameplayStatics.GetAllActorsOfClass` "/Game/ThirdPersonBP/Blueprints/ThirdPersonCharacter.ThirdPersonCharacter_C"))
        (for _array_element _outactors
          (`/Game/ThirdPersonBP/Blueprints/ThirdPersonCharacter.SetHoldingObject` _array_element true)
          (set `self.PlayerHolding` true)))))
  (:`Released`
    (if (`self.CharginThrow`)
      (set `self.CharginThrow` false)
      (`PrimitiveComponent.SetCollisionEnabled` (`self.Sphere`) "QueryOnly")
      (`PrimitiveComponent.SetCollisionEnabled` _pillow "QueryAndPhysics")
      (`SceneComponent.SetVisibility` _pillow true false)
      (`PrimitiveComponent.SetSimulatePhysics` _pillow true)
      (set `self.PlayerHolding` false)
      (`PrimitiveComponent.SetAllPhysicsLinearVelocity` (`self.Pillow`) (* (+ (`self.GetActorForwardVector` (`GameplayStatics.GetPlayerCharacter` 0)) (0.0 0.0 1.0)) (`self.CurrentImpulse`)) false)
      (set `self.Thrown` true)
      (bind _outactors_2 (`GameplayStatics.GetAllActorsOfClass` "/Game/ThirdPersonBP/Blueprints/ThirdPersonCharacter.ThirdPersonCharacter_C"))
      (for _array_element_2 _outactors_2
        (`/Game/ThirdPersonBP/Blueprints/ThirdPersonCharacter.SetHoldingObject` _array_element_2 false)
        (set `self.CurrentImpulse` 0.0)))))

(fn `UserConstructionScript`)